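; BP_P38 is a P-38 aircraft actor that spins its propellers and flies along a straight line.
; Each Tick rolls the Left and Right propeller components in opposite directions at PropellerRotateSpeed.
; The same Tick then moves the actor along world X at a fixed, hardcoded speed, with both rotation and movement scaled by world delta seconds for frame-rate independence.
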(event EventBeginPlay)

(event Collision|EventActorBeginOverlap
  (params (OtherActor :type Actor%20Object%20Reference)))

(event EventTick
  (params (DeltaSeconds :type Float%20%28single-precision%29))
  (Variables|Default|SetDelta%20Seconds DeltaSeconds)
  ;[1 1 1] 왼쪽 프로펠러 회전
  (Transformation|AddLocalRotation (Variables|Default|GetLeft) (Math|Rotator|MakeRotator (* (Utilities|Time|GetWorldDeltaSeconds) (Variables|Default|GetPropellerRotateSpeed)) 0.0 0.0) false false)
  ;[1 1 1] 오른쪽 프로펠러 회전
  (Transformation|AddLocalRotation (Variables|Default|GetRight) (Math|Rotator|MakeRotator (* (Utilities|Time|GetWorldDeltaSeconds) (Variables|Default|GetPropellerRotateSpeed) -1.0) 0.0 0.0) false false)
  ;[1 1 1] 비행기 이동
  (Transformation|AddActorWorldOffset self (Math|Vector|MakeVector (* (Utilities|Time|GetWorldDeltaSeconds) 6e+01) 0.0 0.0)))

(fn ConstructionScript)